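; BP_PlayerEntity is an input relay that forwards player controls to an NGPlayer actor.
; Its Reset, Flip Grav and Move inputs call that actor's reset, gravity flip and movement functions.
; A helper finds the target by casting the entity's root attached actor to NGPlayer, printing a warning if the cast fails.
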(event Input|ActionEvents|InputActionFlipGrav
  (params (Key :type Key%20Structure))
  (:Pressed
    (Default|FlipGravity (CallFunction|GetNGPlayer))))

(event Input|ActionEvents|InputActionReset
  (params (Key :type Key%20Structure))
  (:Pressed
    (Default|Reset (CallFunction|GetNGPlayer))))

(event Input|AxisEvents|InputAxisMove
  (params (AxisValue :type Float%20%28single-precision%29))
  (Default|Move (CallFunction|GetNGPlayer) AxisValue))

(fn ConstructionScript)

(fn GetNGPlayer
  (bind _root (CallFunction|GetRootAttachedActor self))
  (bind _asngplayer (Utilities|Casting|CastToNGPlayer _root)
    (:then
      (return _asngplayer))
    (:CastFailed
      (Development|PrintString "ROOT IS NOT NG ACTOR")
      (return 0))))