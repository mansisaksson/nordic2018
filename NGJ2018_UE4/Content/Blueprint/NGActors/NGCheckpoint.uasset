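; NGCheckpoint is a checkpoint actor that hands a location to the player who touches it.
; When an NGPlayer begins overlapping its Capsule, it calls TakeCheckpoint on that player with the world location of its Pos component.
; Every tick, a visibility line trace runs down the capsule's local up axis and moves the skeletal mesh to the hit point, keeping it on the surface below.
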(event OnComponentBeginOverlap(Capsule)
  (params (OverlappedComponent :type Primitive%20Component%20Object%20Reference) (OtherActor :type Actor%20Object%20Reference) (OtherComp :type Primitive%20Component%20Object%20Reference) (OtherBodyIndex :type Integer) (bFromSweep :type Boolean) (SweepResult :type Hit%20Result%20Structure%20%28by%20ref%29))
  (bind _asngplayer (Utilities|Casting|CastToNGPlayer OtherActor))
  (Default|TakeCheckpoint _asngplayer (Transformation|GetWorldLocation (Variables|Default|GetPos))))

(event EventTick
  (params (DeltaSeconds :type Float%20%28single-precision%29))
  (bind _capsule (Variables|Default|GetCapsule))
  (bind _returnvalue (Transformation|GetWorldLocation _capsule))
  (bind (_outhit _returnvalue_2) (Collision|LineTraceByChannel _returnvalue (+ _returnvalue (* (* (Math|Vector|GetUpVector _capsule) -1.0) 1e+04)) "TraceTypeQuery1" false 0 "None"))
  (if _returnvalue_2
    (Transformation|SetWorldLocation (Variables|Default|GetSkeletalMesh) (.Location (Collision|BreakHitResult _outhit)) false false)))

(fn ConstructionScript)