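; NGPlayer is a physics-driven player actor with flippable gravity, horizontal movement and checkpoint respawn.
; Tick applies gravity as vertical acceleration, and Move adds acceleration along Y.
; Hits set a short-lived IsColliding flag through a retriggerable delay, so gravity flips only during recent contact.
; Reset teleports to the checkpoint or start position and clears velocity; external instances disable physics and skip gravity, checkpoints and reset.
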(event OnComponentHit(Player)
  (params (HitComponent :type Primitive%20Component%20Object%20Reference) (OtherActor :type Actor%20Object%20Reference) (OtherComp :type Primitive%20Component%20Object%20Reference) (NormalImpulse :type Vector :default "0, 0, 0") (Hit :type Hit%20Result%20Structure%20%28by%20ref%29))
  (Variables|Default|SetIs%20Colliding true)
  (Utilities|FlowControl|RetriggerableDelay 0.1)
  (Variables|Default|SetIs%20Colliding false))

(event Custom|Move
  (params (Axis :type Float%20%28single-precision%29))
  (Physics|AddForce (Variables|Default|GetPlayer) (Math|Vector|MakeVector 0.0 (* Axis (Variables|Default|GetMove%20Force)) 0.0) "None" true))

(event Custom|Take%20Checkpoint
  (params (CheckpointPos :type Vector))
  (if (not (Class|NGActor|IsExternal))
    (Variables|Default|SetCheckpointPos CheckpointPos)
    (Variables|Default|SetUse%20checkpoint true)))

(event EventBeginPlay
  (Variables|Default|SetStart%20Pos (Transformation|GetActorLocation))
  (Utilities|FlowControl|Delay 0.0)
  (if (Class|NGActor|IsExternal)
    (Physics|SetSimulatePhysics (Variables|Default|GetPlayer) false)))

(event EventTick
  (params (DeltaSeconds :type Float%20%28single-precision%29))
  (if (not (Class|NGActor|IsExternal))
    (Physics|AddForce (Variables|Default|GetPlayer) (Math|Vector|MakeVector 0.0 0.0 (* (Class|NGSceneManager|GetGravityDir) (Variables|Default|GetGrav%20Strength))) "None" true)))

(fn ConstructionScript)

(fn FlipGravity
  (if (Variables|Default|GetIs%20Colliding)
    (Class|NGSceneManager|FlipGravityDir)))

(fn Reset
  (if (not (Class|NGActor|IsExternal))
    (Transformation|SetActorRelativeLocation (select (Variables|Default|GetUse%20checkpoint) (Variables|Default|GetCheckpointPos) (Variables|Default|GetStart%20Pos)) false true)
    (Class|PrimitiveComponent|SetAllPhysicsLinearVelocity (Variables|Default|GetPlayer) "0, 0, 0" false)))